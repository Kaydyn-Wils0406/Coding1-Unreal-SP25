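; A platform that drops when the player character steps on it, then returns to its starting position.
; An overlap by BP_Custom3rdPersonChar while ready starts an Activated, Falling, Resetting chain, each stage swapping the material.
; Falling enables physics simulation after a delay; resetting disables it and a timeline lerps from the fallen transform back to the one saved at BeginPlay, then re-arms the trigger.
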(event OnComponentBeginOverlap(BoxTringer)
  (params (OverlappedComponent :type Primitive%20Component%20Object%20Reference) (OtherActor :type Actor%20Object%20Reference) (OtherComp :type Primitive%20Component%20Object%20Reference) (OtherBodyIndex :type Integer) (bFromSweep :type Boolean) (SweepResult :type Hit%20Result%20Structure%20%28by%20ref%29))
  (Development|PrintString "Something Hit my trigger!!")
  (if (Variables|Default|GetisReady)
    (Utilities|Casting|CastToBP_Custom3rdPersonChar OtherActor)
    (CallFunction|Activated)))

(event Custom|Activated
  ;[0 1 0.9257 0.5] This changes color to active and waits one second then goes to falling.
  (Development|PrintString "Activated")
  (Rendering|Material|SetMaterial (Variables|Default|GetPlatform) 0 "/Game/Materials/PlatformMaterials/MI_Platform_Activated.MI_Platform_Activated")
  (Variables|Default|SetisReady false) ; We are not ready!!
  (Utilities|FlowControl|Delay (Variables|PlatformSetttings|GetFall%20Delay%20Duration))
  (CallFunction|Falling))

(event Custom|Resetting
  ;[0.05478 1 0.1995 0.5] Comment
  (Development|PrintString "Resetting")
  (Rendering|Material|SetMaterial (Variables|Default|GetPlatform) 0 "/Game/Materials/PlatformMaterials/MI_Platform_Resetting.MI_Platform_Resetting")
  (Variables|Default|SetFallen%20Transform (Transformation|GetWorldTransform (Variables|Default|GetPlatform)))
  (Physics|SetSimulatePhysics (Variables|Default|GetPlatform) false)
  (bind _newtrack_0 (Timeline|ReturnToStart PlayFromStart)
    (:Update
      (Transformation|SetWorldLocationAndRotation (Variables|Default|GetPlatform) (.location (Math|Transform|Lerp(Transform) (Variables|Default|GetFallen%20Transform) (Variables|Default|GetOriginal%20Transform) _newtrack_0)) (.rotation (Math|Transform|Lerp(Transform) (Variables|Default|GetFallen%20Transform) (Variables|Default|GetOriginal%20Transform) _newtrack_0)) false false))
    (:Finished
      (Variables|Default|SetisReady true) ; We are ready now!
      (Rendering|Material|SetMaterial (Variables|Default|GetPlatform) 0 "/Game/Materials/PlatformMaterials/MI_Platform_Ready.MI_Platform_Ready"))))

(event Custom|Falling
  ;[1 0 0.9495 0.5] Comment
  (Development|PrintString "Falling")
  (Rendering|Material|SetMaterial (Variables|Default|GetPlatform) 0 "/Game/Materials/PlatformMaterials/MI_Platform_Falling.MI_Platform_Falling")
  (Physics|SetSimulatePhysics (Variables|Default|GetPlatform) true)
  (Utilities|FlowControl|Delay (Variables|Default|GetDelay%20Duration))
  (CallFunction|Resetting))

(event EventBeginPlay
  (Variables|Default|SetOriginal%20Transform (Transformation|GetWorldTransform (Variables|Default|GetPlatform)))
  (Rendering|Material|SetMaterial (Variables|Default|GetPlatform) 0 "/Game/Materials/PlatformMaterials/MI_Platform_Ready.MI_Platform_Ready"))

(event Collision|EventActorBeginOverlap
  (params (OtherActor :type Actor%20Object%20Reference)))

(event EventTick
  (params (DeltaSeconds :type Float%20%28single-precision%29)))

(fn ConstructionScript)